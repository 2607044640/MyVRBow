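; VR bow held by one motion controller and drawn with a second, whose grab spawns an arrow.
; Tick derives a hold state: unheld drops with physics, two-handed aims the bow along the hands and positions the arrow.
; Two cable components form the string, meeting at a midpoint pulled back by clamped hand distance.
; Leaving the two-handed state fires the arrow through its ProjectileMovement, scaled by draw distance and bow strength.
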(event EventTick
  (params (DeltaSeconds :type Float%20%28single-precision%29))
  (Utilities|FlowControl|Sequence
    (:then_0
      (CallFunction|SetBowState)
      (CallFunction|MidpointSettoEndpoint)
      (CallFunction|SetCableLocation)
      (switch Utilities|FlowControl|Switch|SwitchonBowState (Variables|Default|GetBowState)
        (:NewEnumerator0
          (Transformation|DetachFromActor "KeepWorld" "KeepWorld" "KeepWorld")
          (Physics|SetSimulatePhysics (Variables|Default|GetStaticMesh) true)
          (CallFunction|ReleaseArrow))
        (:NewEnumerator1
          (CallFunction|ReleaseArrow))
        (:NewEnumerator2
          (CallFunction|SetBowRotation)
          (CallFunction|SetArrow)
          (CallFunction|Backup)
          (CallFunction|BpSpawnedArrowLocate))))))

(event EventGrab
  (params (MotionController :type Motion%20Controller%20Component%20Object%20Reference))
  (bind _primarymotioncontroller (Variables|Default|GetPrimaryMotionController)
    (:then
      (if (!= _primarymotioncontroller MotionController)
        (Variables|Default|SetSecondaryMotionController MotionController)
        (Actor|Tick|SetActorTickEnabled true)
        (bind _returnvalue (Game|SpawnActorfromClass "/Game/Blueprints/Bow/BP_Arrow.BP_Arrow_C" (Transformation|GetWorldTransform (Variables|Default|GetSecondaryMotionController)) "Undefined" "MultiplyWithRoot" 0 0))
        (Variables|Default|SetBP_SpawnedArrow _returnvalue)))
    (:else
      (bind _output_get (Variables|Default|SetPrimaryMotionController MotionController))
      (Transformation|AttachComponentToComponent _output_get "None" "SnapToTarget" "SnapToTarget" "KeepWorld" true))))

(event EventRelease
  (params (MotionController :type Motion%20Controller%20Component%20Object%20Reference))
  (if (== (Variables|Default|GetSecondaryMotionController) MotionController)
    (Variables|Default|SetSecondaryMotionController 0)
    (else
      (Variables|Default|SetSecondaryMotionController 0)
      (Variables|Default|SetPrimaryMotionController 0))))

(fn ConstructionScript
  (bind _cable_width (Variables|Default|GetCable%20Width))
  (Variables|/Script/CableComponent.CableComponent|SetCableWidth (Variables|Default|GetCable1) _cable_width)
  (Variables|/Script/CableComponent.CableComponent|SetCableWidth (Variables|Default|GetCable2) _cable_width))

(fn ReleaseArrow
  (bind _bp_spawnedarrow (Variables|Default|GetBP_SpawnedArrow))
  (bind _returnvalue (Actor|GetComponentbyClass _bp_spawnedarrow "/Script/Engine.ProjectileMovementComponent"))
  (if (Variables|Default|GetCanReleaseArrow)
    (Game|Components|ProjectileMovement|SetVelocityinLocalSpace _returnvalue (Math|Vector|MakeVector (* (Variables|Default|GetDistance) (Variables|Default|GetBowStength)) 0.0 0.0))
    (Variables|/Script/Engine.ProjectileMovementComponent|SetProjectileGravityScale _returnvalue 1.0)
    (Variables|Default|SetCanReleaseArrow false)))

(fn SetBowRotation
  (bind _secondarymotioncontroller (Variables|Default|GetSecondaryMotionController))
  (bind _primarymotioncontroller (Variables|Default|GetPrimaryMotionController))
  (bind _returnvalue (Transformation|GetWorldLocation _primarymotioncontroller))
  (bind _returnvalue_2 (Transformation|GetWorldLocation _secondarymotioncontroller))
  (bind _returnvalue_3 (Math|Rotator|FindLookatRotation _returnvalue_2 _returnvalue))
  (Transformation|SetActorRotation (Math|Rotator|MakeRotator (.roll (Transformation|GetWorldRotation _primarymotioncontroller)) (.pitch _returnvalue_3) (.yaw _returnvalue_3))))

(fn SetCableLocation
  (bind _cable2 (Variables|Default|GetCable2))
  (bind _cable1 (Variables|Default|GetCable1))
  (bind _relativelocation (Variables|/Script/Engine.SceneComponent|GetRelativeLocation _cable2))
  (bind _relativelocation_2 (Variables|/Script/Engine.SceneComponent|GetRelativeLocation _cable1))
  (Variables|Default|SetMiddlePoint (+ _relativelocation_2 (* (/ (Math|Vector|Distance(Vector) _relativelocation_2 _relativelocation) 2.0) (Math|Vector|GetForwardVector (Math|Rotator|FindLookatRotation _relativelocation_2 _relativelocation)))))
  (Utilities|IsValid (Variables|Default|GetSecondaryMotionController)
    (:Is%20Valid
      (bind _output_get (Variables|Default|SetDistance (Math|Float|Clamp(Float) (* (Math|Vector|Distance(Vector) (Transformation|GetWorldLocation (Variables|Default|GetPrimaryMotionController)) (Transformation|GetWorldLocation (Variables|Default|GetSecondaryMotionController))) -1.0) (* (Variables|Default|GetClampStengthLength) -1.0))))
      (Variables|Default|SetMiddlePoint (Math|Vector|MakeVector _output_get 0.0 0.0)))))

(fn SetArrow
  (bind _arrow (Variables|Default|GetArrow))
  (Utilities|FlowControl|Sequence
    (:then_0
      (return))
    (:then_1
      (Utilities|IsValid (Variables|Default|GetBP_SpawnedArrow)
        (:Is%20Valid
          (Transformation|SetWorldTransform _arrow (Math|Transform|MakeTransform (Variables|Default|GetMiddlePoint) (Transformation|GetWorldRotation _arrow) "1.000000,1.000000,1.000000") false false))))))

(fn SetBowState
  (Variables|Default|GetPrimaryMotionController
    (:then
      (Variables|Default|GetSecondaryMotionController
        (:then
          (Variables|Default|SetBowState "NewEnumerator2"))
        (:else
          (Variables|Default|SetBowState "NewEnumerator1"))))
    (:else
      (Variables|Default|SetBowState "NewEnumerator0"))))

(fn MidpointSettoEndpoint
  (bind _middlepoint (Variables|Default|GetMiddlePoint))
  (Variables|/Script/CableComponent.CableComponent|SetEndLocation (Variables|Default|GetCable2) _middlepoint)
  (Variables|/Script/CableComponent.CableComponent|SetEndLocation (Variables|Default|GetCable1) _middlepoint))

(fn Backup
  (Variables|Default|SetSecondaryHandPositionBackup (Transformation|GetWorldLocation (Variables|Default|GetSecondaryMotionController)))
  (Variables|Default|SetCanReleaseArrow true))

(fn BpSpawnedArrowLocate
  (Transformation|SetActorTransform (Variables|Default|GetBP_SpawnedArrow) (Math|Transform|MakeTransform (+ (Math|Vector|RotateVector (Variables|Default|GetMiddlePoint) (Transformation|GetWorldRotation (Variables|Default|GetStaticMesh))) (Transformation|GetWorldLocation (Variables|Default|GetStaticMesh))) (Math|Rotator|FindLookatRotation (Transformation|GetWorldLocation (Variables|Default|GetSecondaryMotionController)) (Transformation|GetWorldLocation (Variables|Default|GetStaticMesh))) "1.000000,1.000000,1.000000")))